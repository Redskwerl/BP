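; BP_GetTime attaches to a BP_TimeOfDayManager owner and switches the emissive glow of actors tagged "Turnable" according to time of day.
; After a short BeginPlay delay, a looping five-minute timer reads the manager's time and passes each tagged actor to LightManager.
; LightManager creates dynamic material instances for every static mesh material slot, setting EmissiveScale to off by day, medium at dawn and dusk, and brighter at night.
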(event Custom|CustomEvent_0
  (bind _returnvalue (Class|ConanTimeOfDayManager|GetTimeOfDay (Variables|Default|GetTime%20of%20Day%20Manager)))
  (Variables|Default|SetTime _returnvalue)
  (bind _outactors (Actor|GetAllActorswithTag "Turnable"))
  (for _array_element _outactors
    (CallFunction|LightManager _array_element (Variables|Default|GetTime))))

(event EventBeginPlay
  (Utilities|FlowControl|Delay 0.2)
  (bind _asbp_time_of_day_manager (Utilities|Casting|CastToBP_TimeOfDayManager (Components|GetOwner)))
  (Variables|Default|SetTime%20of%20Day%20Manager _asbp_time_of_day_manager)
  (Utilities|Time|SetTimerbyEvent (delegate Custom|CustomEvent_0) 3e+02 true))

(event EventTick
  (params (DeltaSeconds :type Float%20%28single-precision%29)))

(fn LightManager
  (params (TurnableActor :type Actor%20Object%20Reference) (Time? :type Float%20%28single-precision%29))
  (bind _returnvalue (Actor|GetComponentsByClass TurnableActor "/Script/Engine.StaticMeshComponent"))
  (if (> (Utilities|Array|Length _returnvalue) 0)
    (LocalVariables|SetComponentArray_temp _returnvalue)
    (if (and (>= Time? 6.0) (<= Time? 17.5))
      (for _array_element (LocalVariables|GetComponentArray_temp)
        (for (_ _array_index) (Rendering|Material|GetMaterials _array_element)
          (bind _returnvalue_2 (Rendering|Material|CreateDynamicMaterialInstance _array_element _array_index (Rendering|Material|GetMaterial _array_element _array_index) :!class /Script/Engine.PrimitiveComponent))
          (Rendering|Material|SetScalarParameterValue _returnvalue_2 "EmissiveScale" 0.0 :!class /Script/Engine.MaterialInstanceDynamic)))
      (elif (or (and (>= Time? 17.6) (<= Time? 2e+01)) (and (>= Time? 5.0) (<= Time? 5.99)))
        (for _array_element_2 (LocalVariables|GetComponentArray_temp)
          (for (_ _array_index_2) (Rendering|Material|GetMaterials _array_element_2)
            (bind _returnvalue_3 (Rendering|Material|CreateDynamicMaterialInstance _array_element_2 _array_index_2 (Rendering|Material|GetMaterial _array_element_2 _array_index_2) :!class /Script/Engine.PrimitiveComponent))
            (Rendering|Material|SetScalarParameterValue _returnvalue_3 "EmissiveScale" 1.0 :!class /Script/Engine.MaterialInstanceDynamic)))
        (else
          (for _array_element_3 (LocalVariables|GetComponentArray_temp)
            (for (_ _array_index_3) (Rendering|Material|GetMaterials _array_element_3)
              (bind _returnvalue_4 (Rendering|Material|CreateDynamicMaterialInstance _array_element_3 _array_index_3 (Rendering|Material|GetMaterial _array_element_3 _array_index_3) :!class /Script/Engine.PrimitiveComponent))
              (Rendering|Material|SetScalarParameterValue _returnvalue_4 "EmissiveScale" 2.0 :!class /Script/Engine.MaterialInstanceDynamic))))))
    (else
      (return))))